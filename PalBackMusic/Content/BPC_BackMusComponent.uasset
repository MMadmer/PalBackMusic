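; Actor component that plays 2D day or night background music for its owning PalCharacter, destroying itself on any other owner.
; After a short clock-derived delay, it spawns the track for the current time and binds day/night and battle-mode delegates.
; Day changes fade out, swap cues and fade in, while battles lower volume then pause playback, restoring it afterwards.
; Pre-created looping timers, paused and unpaused, sequence these delayed steps.
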(event `self.ReceiveBeginPlay`
  (bind _returnvalue (/ (`KismetMathLibrary.Conv_Int64ToDouble` (`KismetMathLibrary.Conv_DoubleToInt64` (`KismetStringLibrary.Conv_StringToDouble` (`KismetStringLibrary.Right` (`KismetStringLibrary.Conv_DoubleToString` (`.PartialSeconds` (`GameplayStatics.GetAccurateRealTime`))) 1)))) 10.0))
  (`self.SetComponentTickEnabled` false)
  (bind _aspal_character (cast `PalCharacter` (`self.GetOwner`))
    (:`then`
      (set `self.Owner` _aspal_character)
      (`KismetSystemLibrary.K2_SetTimerDelegate` (delegate `RandomMusic`) _returnvalue false _returnvalue 1.0))
    (:`CastFailed`
      (`self.K2_DestroyComponent`))))

(event `RandomMusic`
  (bind _returnvalue (`GameplayStatics.SpawnSound2D` (select `EPalOneDayTimeType` (`PalTimeManager.GetCurrentDayTimeType` (`PalUtility.GetTimeManager`)) :`Undefined` "/Game/Mods/PalBackMusic_P/Music/M_Day_BackgroundCue.M_Day_BackgroundCue" :`Day` "/Game/Mods/PalBackMusic_P/Music/M_Day_BackgroundCue.M_Day_BackgroundCue" :`Night` "/Game/Mods/PalBackMusic_P/Music/M_Night_BackgroundCue.M_Night_BackgroundCue" :!type "SoundBase Object Reference") 1.0 1.0 0.0 null false false))
  (bind _output_get (set `self.BackgroundSound` _returnvalue))
  (`AudioComponent.SetVolumeMultiplier` _output_get (`self.MaxVolume`))
  (`self.AssignBattle`)
  (`self.AssignDay`))

(event `AssignDay`
  (bind _returnvalue (`PalUtility.GetTimeManager`))
  (bind _returnvalue_2 (/ (`self.DayChangeTime`) 2.0))
  (bind _returnvalue_3 (/ (`self.DayChangeTime`) 2.0))
  (bind _returnvalue_4 (`KismetSystemLibrary.K2_SetTimerDelegate` (delegate `OnNightStart`) _returnvalue_3 true _returnvalue_3))
  (bind _output_get (set `self.DayEndTimerHandle` _returnvalue_4))
  (`KismetSystemLibrary.K2_PauseTimerHandle` _output_get)
  (bind _returnvalue_5 (`KismetSystemLibrary.K2_SetTimerDelegate` (delegate `OnNightEnd`) _returnvalue_2 true _returnvalue_2))
  (bind _output_get_2 (set `self.DayStartTimerHandle` _returnvalue_5))
  (`KismetSystemLibrary.K2_PauseTimerHandle` _output_get_2)
  (add `PalTimeManager.OnNightStartDelegate` _returnvalue (delegate `OnDayEnd`))
  (add `PalTimeManager.OnNightEndDelegate` _returnvalue (delegate `OnDayStart`))
  (add `PalTimeManager.OnNightEndDelegate` (`PalUtility.GetTimeManager`) (delegate `OnDayStart`))
  (add `PalTimeManager.OnNightSkipDelegate` (`PalUtility.GetTimeManager`) (delegate `OnDayStart`)))

(event `OnDayEnd`
  (`KismetSystemLibrary.K2_PauseTimerHandle` (`self.DayStartTimerHandle`))
  (`KismetSystemLibrary.K2_UnPauseTimerHandle` (`self.DayEndTimerHandle`))
  (`AudioComponent.FadeOut` (`self.BackgroundSound`) (/ (`self.DayChangeTime`) 2.0) 0.0 "Logarithmic"))

(event `OnNightStart`
  (bind _backgroundsound (`self.BackgroundSound`))
  (`KismetSystemLibrary.K2_PauseTimerHandle` (`self.DayEndTimerHandle`))
  (`AudioComponent.SetSound` _backgroundsound "/Game/Mods/PalBackMusic_P/Music/M_Night_BackgroundCue.M_Night_BackgroundCue")
  (`AudioComponent.FadeIn` _backgroundsound (/ (`self.DayChangeTime`) 2.0) (`self.MaxVolume`) 0.0 "Logarithmic"))

(event `OnDayStart`
  (`KismetSystemLibrary.K2_PauseTimerHandle` (`self.DayEndTimerHandle`))
  (`KismetSystemLibrary.K2_UnPauseTimerHandle` (`self.DayStartTimerHandle`))
  (`AudioComponent.FadeOut` (`self.BackgroundSound`) (/ (`self.DayChangeTime`) 2.0) 0.0 "Logarithmic"))

(event `OnNightEnd`
  (bind _backgroundsound (`self.BackgroundSound`))
  (`KismetSystemLibrary.K2_PauseTimerHandle` (`self.DayStartTimerHandle`))
  (`AudioComponent.SetSound` _backgroundsound "/Game/Mods/PalBackMusic_P/Music/M_Day_BackgroundCue.M_Day_BackgroundCue")
  (`AudioComponent.FadeIn` _backgroundsound (/ (`self.DayChangeTime`) 2.0) (`self.MaxVolume`) 0.0 "Logarithmic"))

(event `AssignBattle`
  (bind _battlestarttime (`self.BattleStartTime`))
  (bind _battleendtime (`self.BattleEndTime`))
  (bind _returnvalue (`KismetSystemLibrary.K2_SetTimerDelegate` (delegate `OnBattleStart`) _battlestarttime true _battlestarttime))
  (bind _output_get (set `self.BattleStartTimerHandle` _returnvalue))
  (`KismetSystemLibrary.K2_PauseTimerHandle` _output_get)
  (bind _returnvalue_2 (`KismetSystemLibrary.K2_SetTimerDelegate` (delegate `OnBattleEnd`) _battleendtime true _battleendtime))
  (bind _output_get_2 (set `self.BattleEndTimerHandle` _returnvalue_2))
  (`KismetSystemLibrary.K2_PauseTimerHandle` _output_get_2)
  (add `PalCharacter.OnChangeBattleModeDelegate` (`self.Owner`) (delegate `OnChangeBattleMode`)))

(event `OnBattleStart`
  (`AudioComponent.SetPaused` (`self.BackgroundSound`) true))

(event `OnBattleEnd`
  (`AudioComponent.SetPaused` (`self.BackgroundSound`) false))

(event `OnChangeBattleMode`
  (params (bIsBattleMode :type Boolean))
  (if bIsBattleMode
    (`KismetSystemLibrary.K2_PauseTimerHandle` (`self.BattleEndTimerHandle`))
    (`KismetSystemLibrary.K2_UnPauseTimerHandle` (`self.BattleStartTimerHandle`))
    (`AudioComponent.AdjustVolume` (`self.BackgroundSound`) (`self.BattleStartTime`) 0.01 "Logarithmic")
    (else
      (`KismetSystemLibrary.K2_PauseTimerHandle` (`self.BattleStartTimerHandle`))
      (`KismetSystemLibrary.K2_UnPauseTimerHandle` (`self.BattleEndTimerHandle`))
      (`AudioComponent.AdjustVolume` (`self.BackgroundSound`) (`self.BattleEndTime`) (`self.MaxVolume`) "Logarithmic"))))